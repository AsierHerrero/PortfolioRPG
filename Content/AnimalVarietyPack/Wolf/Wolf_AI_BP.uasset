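; Wolf_AI_BP is the AI controller for the wolf, running Wolf_BT and caching the controlled Wolf_BP on BeginPlay.
; AI Perception updates ask each sensed actor whether it is an enemy through an IsEnemy message, storing matches as CurrentEnemy and in the Blackboard's Enemy key.
; Losing perception of the current enemy clears that key but leaves CurrentEnemy set.
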(event `self.ReceiveBeginPlay`
  (`self.RunBehaviorTree` "/Game/AnimalVarietyPack/Wolf/Wolf_BT.Wolf_BT")
  (bind _aswolf_bp (cast `/Game/AnimalVarietyPack/Wolf/Wolf_BP` (`self.K2_GetPawn`)))
  (set `self.My Pawn` _aswolf_bp))

(event `self.AIPerception.OnTargetPerceptionUpdated`
  (params (Actor :type "Actor Object Reference") (Stimulus :type "AIStimulus Structure"))
  (bind _blackboard (`self.Blackboard`))
  (if (`.bSuccessfullySensed` (break `AIStimulus` Stimulus))
    (bind _enemy (message `/Game/AnimalVarietyPack/Wolf/BPI_Wolf.IsEnemy?` Actor))
    (if _enemy
      (set `self.Current Enemy` Actor)
      (`BlackboardComponent.SetValueAsObject` _blackboard "Enemy" Actor))
    (elif (== Actor (`self.Current Enemy`))
      (`BlackboardComponent.ClearValue` _blackboard "Enemy"))))

(fn `UserConstructionScript`)
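; BP_Pig is a farm animal pawn that wanders around on its own.
; From BeginPlay it waits a random few seconds, then sets its walk speed and uses AIMoveTo to reach a random reachable point near its current location.
; A successful move schedules the next roam, forming an endless idle-and-walk loop; a failed move has no handler, so the loop stops there.
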(event `self.ReceiveBeginPlay`
  (`self.DecideNextAction` false))

(event `DecideNextAction`
  (params (`SkipDelay?` :type Boolean))
  (if (not `SkipDelay?`)
    (`KismetSystemLibrary.Delay` (`KismetMathLibrary.Conv_IntToDouble` (`KismetMathLibrary.RandomIntegerInRange` 1 5))))
  (`self.RandomRoam`))

(event `RandomRoam`
  ;[1 1 1] RandomRoam
  (set `CharacterMovementComponent.MaxWalkSpeed` 150.0 (`self.CharacterMovement`))
  (`|AIMoveTo` self (`NavigationSystemV1.K2_GetRandomReachablePointInRadius` (`self.K2_GetActorLocation`) 500.0 null null) null
    (:`OnSuccess`
      (`self.DecideNextAction` false))))

(fn `UserConstructionScript`)